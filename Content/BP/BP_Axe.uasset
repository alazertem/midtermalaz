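; BP_Axe is an axe trap that swings and damages the third-person character on overlap unless that player holds the AxeKey.
; BeginPlay caches the player and computes the swing's pitch-offset end rotation.
; Overlap deducts health immediately and latches Triggered, making Tick play the Swing timeline that lerps the axe's relative rotation.
; Tick also polls the player's AxeKey and destroys the actor once it is set.
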(event Collision|EventActorBeginOverlap
  (params (OtherActor :type Actor%20Object%20Reference))
  (bind _asbp_third_person_character (Utilities|Casting|CastToBP_ThirdPersonCharacter OtherActor))
  (if (not (Variables|/Game/ThirdPerson/Blueprints/BP_ThirdPersonCharacter.BP_ThirdPersonCharacter_C|GetAxeKey _asbp_third_person_character))
    (Variables|Default|Settriggered true)
    (Variables|/Game/ThirdPerson/Blueprints/BP_ThirdPersonCharacter.BP_ThirdPersonCharacter_C|SetHealth _asbp_third_person_character (- (Variables|/Game/ThirdPerson/Blueprints/BP_ThirdPersonCharacter.BP_ThirdPersonCharacter_C|GetHealth (Variables|Default|Getplayer)) 3e+01))))

(event EventBeginPlay
  (bind _axe (Variables|Default|GetAxe))
  (bind _relativerotation (Variables|/Script/Engine.SceneComponent|GetRelativeRotation _axe))
  (bind (_roll _pitch _yaw) (Math|Rotator|BreakRotator _relativerotation))
  (bind _returnvalue (Actor|GetActorOfClass "/Game/ThirdPerson/Blueprints/BP_ThirdPersonCharacter.BP_ThirdPersonCharacter_C"))
  (Variables|Default|Setplayer _returnvalue)
  (Variables|Default|SetCurrentPosition _relativerotation)
  (Variables|Default|SetSwingTo (Math|Rotator|MakeRotator _roll (+ _pitch 2.4e+02) _yaw)))

(event EventTick
  (params (DeltaSeconds :type Float%20%28single-precision%29))
  (if (Variables|/Game/ThirdPerson/Blueprints/BP_ThirdPersonCharacter.BP_ThirdPersonCharacter_C|GetAxeKey (Variables|Default|Getplayer))
    (Actor|DestroyActor)
    (elif (Variables|Default|Gettriggered)
      (bind _swingaxe (Timeline|Swing Play)
        (:Update
          (Transformation|SetRelativeRotation (Variables|Default|GetAxe) (Math|Rotator|Lerp(Rotator) (Variables|Default|GetCurrentPosition) (Variables|Default|GetSwingTo) _swingaxe) false false))))))

(fn ConstructionScript)