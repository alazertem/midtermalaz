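; BP_Spikes is a spike trap actor that damages the third-person character when it overlaps.
; If the character lacks the SpikeKey, the Spikes component jumps up along relative Z and the character's Health is reduced directly by a fixed amount.
; After a short Delay the spikes drop back by the same offset, with instant transform changes rather than animation.
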(event EventBeginPlay)

(event Collision|EventActorBeginOverlap
  (params (OtherActor :type Actor%20Object%20Reference))
  (bind _spikes (Variables|Default|GetSpikes))
  (bind _spikes_2 (Variables|Default|GetSpikes))
  (bind _returnvalue (Transformation|GetRelativeTransform _spikes))
  (bind _returnvalue_2 (Transformation|GetRelativeTransform _spikes_2))
  (bind _asbp_third_person_character (Utilities|Casting|CastToBP_ThirdPersonCharacter OtherActor))
  (if (not (Variables|/Game/ThirdPerson/Blueprints/BP_ThirdPersonCharacter.BP_ThirdPersonCharacter_C|GetSpikeKey _asbp_third_person_character))
    (Transformation|SetRelativeTransform _spikes_2 (Math|Transform|MakeTransform (Math|Vector|MakeVector (.x (.location _returnvalue_2)) (.y (.location _returnvalue_2)) (+ (.z (.location _returnvalue_2)) 2e+02)) (.rotation _returnvalue_2) (.scale _returnvalue_2)) false false)
    (Variables|/Game/ThirdPerson/Blueprints/BP_ThirdPersonCharacter.BP_ThirdPersonCharacter_C|SetHealth _asbp_third_person_character (- (Variables|/Game/ThirdPerson/Blueprints/BP_ThirdPersonCharacter.BP_ThirdPersonCharacter_C|GetHealth _asbp_third_person_character) 2e+01))
    (Utilities|FlowControl|Delay 2.0)
    (Transformation|SetRelativeTransform _spikes (Math|Transform|MakeTransform (Math|Vector|MakeVector (.x (.location _returnvalue)) (.y (.location _returnvalue)) (+ (.z (.location _returnvalue)) -2e+02)) (.rotation _returnvalue) (.scale _returnvalue)) false false)))

(event EventTick
  (params (DeltaSeconds :type Float%20%28single-precision%29)))

(fn ConstructionScript)